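; Photo-booth actor that captures high-res screenshots of a character mesh from four preset camera positions.
; The construction script sets the mesh and aims each position at its bounds center; BeginPlay loads materials and skeleton animations, then stops on the selected animation.
; Each L press moves the single camera to the next position and saves a numbered screenshot.
; After a successful shot, a camera index of exactly 3 triggers a material swap.
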(event `Key|L`
  (params (Key :type "Key Structure"))
  (bind _camera (`self.Camera`))
  (bind _fileindex (`self.FileIndex`))
  (bind _currentcameraindex (`self.CurrentCameraIndex`))
  (bind _returnvalue (`KismetStringLibrary.Concat_StrStr` (`self.OutputPath`) (`KismetStringLibrary.Conv_IntToString` _fileindex)))
  (:`Pressed`
    (bind _result (`/Engine/EditorBlueprintResources/StandardMacros.IncrementInt` _currentcameraindex)
      (:`  `
        (bind _output (`|GetArrayItem` (`|MakeArray` (`self.CameraPos1`) (`self.CameraPos2`) (`self.CameraPos3`) (`self.CameraPos0`)) (mod _result 4)))
        ;[1 1 1] Change ViewTarget
        (`SceneComponent.K2_SetWorldLocation` _camera (`SceneComponent.K2_GetComponentLocation` _output) false false)
        (`SceneComponent.K2_SetWorldRotation` _camera (`SceneComponent.K2_GetComponentRotation` _output) false false)
        (`PlayerController.SetViewTargetWithBlend` (`GameplayStatics.GetPlayerController` 0) self 0.0 "VTBlend_Linear" 0.0 false)
        ;[1 1 1] Take ScreenShot
        (if (`AutomationBlueprintFunctionLibrary.TakeHighResScreenshot` 0 0 _returnvalue null)
          (`KismetSystemLibrary.PrintString` (`KismetStringLibrary.Concat_StrStr` _returnvalue " Screenshot has been taken."))
          (`/Engine/EditorBlueprintResources/StandardMacros.IncrementInt` _fileindex
            (:`  `
              ;[1 1 1] Change Material
              (`/Engine/EditorBlueprintResources/StandardMacros.CompareInt` _currentcameraindex 3
                (:`==`
                  (bind _asmaterial_interface (cast `MaterialInterface` (`|GetArrayItem` (`self.AllMaterials`) (`self.SourceMaterialIndex`))))
                  (`PrimitiveComponent.SetMaterial` (`self.MainCharacter`) (`self.TargetMaterialIndex`) _asmaterial_interface))))))))))

(event `self.ReceiveBeginPlay`
  (bind _maincharacter (`self.MainCharacter`))
  (`self.EnableInput` (`GameplayStatics.GetPlayerController` 0))
  ;[1 1 1] Load All Materials
  (bind _returnvalue (`ObjectLibrary_BP.LoadObjectLibrary` (`self.MaterialPath`)))
  (set `self.AllMaterials` _returnvalue)
  ;[1 1 1] Load All Animations
  (bind _returnvalue_2 (`ObjectLibrary_BP.LoadAllAnimationSequenceForSkeleton` (`SkeletalMesh.Skeleton` (`SkinnedMeshComponent.SkeletalMesh` (`self.MainCharacter`)))))
  (bind _output_get (set `self.AllAnimations` _returnvalue_2))
  (bind _output (`|GetArrayItem` _output_get (`self.AnimationIndex`)))
  ;[1 1 1] Set First Animation
  (`SkeletalMeshComponent.PlayAnimation` _maincharacter _output false)
  (`SkeletalMeshComponent.Stop` _maincharacter)
  (set `self.CurrentAnimation` _output))

(fn `UserConstructionScript`
  (bind _maincharacter (`self.MainCharacter`))
  (bind _camerapos3 (`self.CameraPos3`))
  (bind _camerapos0 (`self.CameraPos0`))
  (bind _camerapos1 (`self.CameraPos1`))
  (bind _camerapos2 (`self.CameraPos2`))
  (bind _origin (`KismetSystemLibrary.GetComponentBounds` _maincharacter))
  (`SkinnedMeshComponent.SetSkinnedAssetAndUpdate` _maincharacter (`self.MainChar`) true)
  ;[1 1 1] Look Main Character
  (`SceneComponent.K2_SetWorldRotation` _camerapos1 (`KismetMathLibrary.FindLookAtRotation` (`SceneComponent.K2_GetComponentLocation` _camerapos1) _origin) false false)
  (`SceneComponent.K2_SetWorldRotation` _camerapos2 (`KismetMathLibrary.FindLookAtRotation` (`SceneComponent.K2_GetComponentLocation` _camerapos2) _origin) false false)
  (`SceneComponent.K2_SetWorldRotation` _camerapos3 (`KismetMathLibrary.FindLookAtRotation` (`SceneComponent.K2_GetComponentLocation` _camerapos3) _origin) false false)
  (`SceneComponent.K2_SetWorldRotation` _camerapos0 (`KismetMathLibrary.FindLookAtRotation` (`SceneComponent.K2_GetComponentLocation` _camerapos0) _origin) false false))